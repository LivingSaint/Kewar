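; Pickup actor, named as the master pickup, that bobs in place and destroys itself when an actor tagged Player overlaps its trigger.
; A MoveUp timeline offsets the root from the location saved at BeginPlay, with a FlipFlop on Finished alternating reverse and forward play to loop the motion.
; The construction script snaps the root to world Y zero, keeping the pickup on the XZ plane.
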(event OnComponentBeginOverlap(PickUpTrigger)
  (params (OverlappedComponent :type Primitive%20Component%20Object%20Reference) (OtherActor :type Actor%20Object%20Reference) (OtherComp :type Primitive%20Component%20Object%20Reference) (OtherBodyIndex :type Integer) (bFromSweep :type Boolean) (SweepResult :type Hit%20Result%20Structure%20%28by%20ref%29))
  (if (Actor|ActorHasTag OtherActor "Player")
    (Actor|DestroyActor)))

(event Custom|StartMoveUp
  (bind _moveup (Timeline|MoveUp Play)
    (:Update
      (Transformation|SetWorldLocation (Variables|Default|GetDefaultSceneRoot) (+ _moveup (Variables|Default|GetvInitialLocation)) false false))
    (:Finished
      (Utilities|FlowControl|FlipFlop
        (:A
          (CallFunction|StartMoveDown))
        (:B
          (CallFunction|StartMoveUp))))))

(event Custom|StartMoveDown
  (bind _moveup (Timeline|MoveUp Reverse)
    (:Update
      (Transformation|SetWorldLocation (Variables|Default|GetDefaultSceneRoot) (+ _moveup (Variables|Default|GetvInitialLocation)) false false))
    (:Finished
      (Utilities|FlowControl|FlipFlop
        (:A
          (CallFunction|StartMoveDown))
        (:B
          (CallFunction|StartMoveUp))))))

(event EventBeginPlay
  (Variables|Default|SetvInitialLocation (Transformation|GetWorldLocation (Variables|Default|GetDefaultSceneRoot)))
  (CallFunction|StartMoveUp))

(fn ConstructionScript
  (CallFunction|LockYAxis()))

(fn LockYAxis()
  (bind _defaultsceneroot (Variables|Default|GetDefaultSceneRoot))
  (bind _returnvalue (Transformation|GetWorldLocation _defaultsceneroot))
  (bind (_x _y _z) (Math|Vector|BreakVector _returnvalue))
  (Transformation|SetWorldLocation (Variables|Default|GetDefaultSceneRoot) (Math|Vector|MakeVector _x 0.0 _z) false true))