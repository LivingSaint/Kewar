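; Blueprint function LockYAxis that snaps an object onto a fixed Y plane according to its environment type, keeping its X and Z.
; Enemies have their capsule component moved to the zero Y plane, as do environment and interactable objects through their scene component.
; Background objects are pushed to one of three evenly spaced negative Y depths chosen by layer level.
; Each move is an unswept teleport in world space.
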(fn LockYAxis
  (params (eGetEnviromentType :type eEnviromentTypes%20Enum) (GetCapsuleComponent :type Capsule%20Component%20Object%20Reference) (GetSceneComponent :type Scene%20Component%20Object%20Reference) (iLayerLevel :type Integer))
  (bind _returnvalue (Transformation|GetWorldLocation GetSceneComponent))
  (bind _returnvalue_2 (Transformation|GetWorldLocation GetCapsuleComponent))
  (bind _returnvalue_3 (Transformation|GetWorldLocation GetSceneComponent))
  (bind (_x _y _z) (Math|Vector|BreakVector _returnvalue))
  (bind (_x_2 _y_2 _z_2) (Math|Vector|BreakVector _returnvalue_3))
  (bind (_x_3 _y_3 _z_3) (Math|Vector|BreakVector _returnvalue_2))
  (switch Utilities|FlowControl|Switch|SwitchoneEnviromentTypes eGetEnviromentType
    (:NewEnumerator1
      (Transformation|SetWorldLocation GetCapsuleComponent (Math|Vector|MakeVector _x_3 0.0 _z_3) false true))
    (:NewEnumerator4
      (Transformation|SetWorldLocation GetSceneComponent (Math|Vector|MakeVector _x_2 0.0 _z_2) false true))
    (:NewEnumerator2
      (switch int iLayerLevel
        (:0
          (LocalVariables|SetfBackgroundLayer -1e+01))
        (:1
          (LocalVariables|SetfBackgroundLayer -2e+01))
        (:2
          (LocalVariables|SetfBackgroundLayer -3e+01)))
      (Transformation|SetWorldLocation GetSceneComponent (Math|Vector|MakeVector _x (LocalVariables|GetfBackgroundLayer) _z) false true)))
  (return))