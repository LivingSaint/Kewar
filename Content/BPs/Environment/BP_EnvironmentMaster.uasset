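; BP_EnvironmentMaster is an environment actor, apparently a master for environment pieces, that displays a configurable Paper2D sprite.
; Its construction script passes the environment type, layer level and root component to LockYAxis, defined outside this file, then assigns the chosen sprite to PutSpriteHere.
; Getters and setters expose the environment type and layer level, and the event graph holds no active logic.
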(event EventBeginPlay)

(event Collision|EventActorBeginOverlap
  (params (OtherActor :type Actor%20Object%20Reference)))

(event EventTick
  (params (DeltaSeconds :type Float%20%28single-precision%29)))

(fn ConstructionScript
  (CallFunction|LockYAxis (Variables|Environment|Enums|GeteEnvironmentType) 0 (Variables|Default|GetDefaultSceneRoot) (Environment|Getters|GetiLayerLevel))
  (Environment|Setters|SetSprite))

(fn SetSprite
  (Rendering|Components|Sprite|SetSprite (Variables|Default|GetPutSpriteHere) (Variables|Environment|Sprite|Getps_SetSprite)))

(fn SeteEnvironmentType
  (params (eEnvironmentType :type eEnviromentTypes%20Enum))
  (Variables|Environment|Enums|SeteEnvironmentType eEnvironmentType))

(fn GetEnvironmentType
  (return (Variables|Environment|Enums|GeteEnvironmentType)))

(fn SetiLayerLevel
  (params (iLayerLevel :type Integer))
  (Variables|Environment|Ints|SetiLayerLevel iLayerLevel))

(fn GetiLayerLevel
  (return (Variables|Environment|Ints|GetiLayerLevel)))