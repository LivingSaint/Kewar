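; Moving environment actor that carries an enemy and shuttles between its original position and MoveToPoint until that enemy dies.
; BeginPlay spawns the enemy, flags it as environmental, binds its death event and starts the delayed movement loop.
; The enemy's class display name picks its attach socket on PutSpriteHere.
; Death is checked between eased MoveComponentTo legs, then PivotPoint settles at MoveToPoint lowered by the bridge offset.
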(event Custom|StartMoving
  (bind _movetopoint (Variables|Default|GetMoveToPoint))
  (bind _fmovetotime (Variables|MovEnv|Floats|GetfMoveToTime))
  (bind _returnvalue (Transformation|GetWorldLocation _movetopoint))
  (bind (_x _y _z) (Math|Vector|BreakVector _returnvalue))
  (if (Variables|Default|GetbISEnemydead?)
    (Components|MoveComponentTo (Variables|Default|GetPivotPoint) (- (Math|Vector|MakeVector _x _y (- _z (Variables|MovEnv|Floats|GetfBridgeLocation))) (Transformation|GetWorldLocation (Variables|Default|GetDefaultSceneRoot))) "0, 0, 0" true true 1.0 false :!label _label)
    (else
      (Components|MoveComponentTo (Variables|Default|GetPivotPoint) (- (Transformation|GetWorldLocation (Variables|Default|GetMoveToPoint)) (Transformation|GetWorldLocation (Variables|Default|GetDefaultSceneRoot))) "0, 0, 0" true true _fmovetotime false)
      (Utilities|FlowControl|Delay _fmovetotime)
      (if (Variables|Default|GetbISEnemydead?)
        (goto _label)
        (else
          (Components|MoveComponentTo (Variables|Default|GetPivotPoint) (Getters|GetOriginalLocation()) "0, 0, 0" true true _fmovetotime false)
          (Utilities|FlowControl|Delay _fmovetotime)
          (CallFunction|StartMoving))))))

(event Custom|StopMoving
  (params (NewParam :type Boolean))
  (Variables|Default|SetbISEnemydead? NewParam)
  (EventDispatchers|UnbindEventfromIsDead (.AsBP%20Enemy%20Parent (Utilities|Casting|CastToBP_EnemyParent (Variables|Default|GetobjEnemyReference))) (delegate Custom|StopMoving)))

(event EventBeginPlay
  (Variables|Default|SetbISEnemydead? false)
  (CallFunction|Spawn&AttachEnemy() (Variables|MovEnv|Actor|GetaEnemySpawn))
  (Default|SetbIsEnvironment() (.AsBP%20Enemy%20Parent (Utilities|Casting|CastToBP_EnemyParent (Variables|Default|GetobjEnemyReference))) true)
  (EventDispatchers|BindEventtoIsDead (.AsBP%20Enemy%20Parent (Utilities|Casting|CastToBP_EnemyParent (Variables|Default|GetobjEnemyReference))) (delegate Custom|StopMoving))
  (Utilities|FlowControl|Delay (Variables|MovEnv|Floats|GetfStartDelay))
  (CallFunction|StartMoving))

(fn ConstructionScript
  (|CallParentFunction)
  (Setters|SetOriginalLocation()))

(fn SetOriginalLocation()
  (Variables|Default|SetvOriginalLocation (Variables|/Script/Engine.SceneComponent|GetRelativeLocation (Variables|Default|GetPivotPoint))))

(fn GetOriginalLocation()
  (return (Variables|Default|GetvOriginalLocation)))

(fn Spawn&AttachEnemy()
  (params (aGetEnemySpawn :type Actor%20Class%20Reference))
  (bind _putspritehere (Variables|Default|GetPutSpriteHere))
  (bind _returnvalue (Transformation|GetWorldTransform _putspritehere))
  (bind (_location _rotation) (Math|Transform|BreakTransform _returnvalue))
  (bind (_x _y _z) (Math|Vector|BreakVector _location))
  (bind _returnvalue_2 (Game|SpawnActorfromClass aGetEnemySpawn (Math|Transform|MakeTransform (Math|Vector|MakeVector _x _y (- _z 1e+02)) _rotation "1.000000,1.000000,1.000000") "Undefined" 0 0))
  (bind _output_get (Variables|Default|SetobjEnemyReference _returnvalue_2))
  (switch string (Utilities|GetClassDisplayName aGetEnemySpawn)
    (:Default
      (Development|PrintString (Utilities|String|Append "Switch in:" "[Spawn&AttachEnemy]" "Inside blueprint: " (Utilities|GetDisplayName self) "Has defaulted")))
    (:BP_DownArrow_C
      (LocalVariables|SetiGetBone 0)
      (Transformation|AttachComponentToComponent _returnvalue_2 _putspritehere (Utilities|Array|Get(acopy) (Transformation|GetAllSocketNames _putspritehere) (LocalVariables|GetiGetBone)) "SnapToTarget" "KeepRelative" "SnapToTarget" true :!label _label)
      (Transformation|SetActorScale3D _output_get "1.000000,1.000000,1.000000"))
    (:BP_UpArrow_C
      (LocalVariables|SetiGetBone 1)
      (goto _label))
    (:BP_LeftnRightArrows_C
      (LocalVariables|SetiGetBone 2)
      (goto _label))))

(fn GetInitialLocation())

(fn SetfBridgeLocation()
  (params (fBridgeLocation :type Float%20%28single-precision%29))
  (Variables|MovEnv|Floats|SetfBridgeLocation fBridgeLocation))