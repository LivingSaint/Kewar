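; Arrow-key enemy character that patrols along the X axis and leaps at the player, with left and right variants set in construction.
; A looping timer moves it and counts ticks, reversing at range limits.
; While a Player-tagged actor is in its box, another timer checks attack readiness, pauses patrol and launches an impulse, or runs cooldown.
; A capsule hit passing the Player tag check during an attack resumes patrol.
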(event OnComponentBeginOverlap(Box)
  (params (OverlappedComponent :type Primitive%20Component%20Object%20Reference) (OtherActor :type Actor%20Object%20Reference) (OtherComp :type Primitive%20Component%20Object%20Reference) (OtherBodyIndex :type Integer) (bFromSweep :type Boolean) (SweepResult :type Hit%20Result%20Structure%20%28by%20ref%29))
  (if (Actor|ActorHasTag OtherActor "Player")
    (bind _returnvalue (Utilities|Time|SetTimerbyEvent (delegate Custom|DetectPlayerL/R) 0.1 true))
    (Variables|Powers|Detection|TimeHandles|SetthDectectPlayerL/R _returnvalue)))

(event OnComponentEndOverlap(Box)
  (params (OverlappedComponent :type Primitive%20Component%20Object%20Reference) (OtherActor :type Actor%20Object%20Reference) (OtherComp :type Primitive%20Component%20Object%20Reference) (OtherBodyIndex :type Integer))
  (if (Actor|ActorHasTag OtherActor "Player")
    (Utilities|Time|PauseTimerbyHandle (Variables|Powers|Detection|TimeHandles|GetthDectectPlayerL/R))))

(event OnComponentHit(CapsuleComponent)
  (params (HitComponent :type Primitive%20Component%20Object%20Reference) (OtherActor :type Actor%20Object%20Reference) (OtherComp :type Primitive%20Component%20Object%20Reference) (NormalImpulse :type Vector :default "0, 0, 0") (Hit :type Hit%20Result%20Structure%20%28by%20ref%29))
  (if (Components|ComponentHasTag HitComponent "Player")
    (if (Variables|Default|GetbIsAttacking?)
      (Variables|Default|SetbIsAttacking? false)
      (Utilities|Time|UnpauseTimerbyHandle (Variables|Movement|Timers|GetthMoveL/R)))))

(event Custom|MoveRight
  (Movement|MoveLeft/Right() (Variables|Movement|Floats|GetfMoveL/RDirection)))

(event Custom|DetectPlayerL/R
  (if (Variables|Default|GetbCanAttack?)
    (bind _vgetplayerlocation (CallFunction|DetectionDirection() (Variables|Default|GetvDetectionDirection)))
    (Utilities|Time|PauseTimerbyHandle (Variables|Movement|Timers|GetthMoveL/R))
    (Utilities|FlowControl|Delay 1.0)
    (Powers|SetChargetoLocation() _vgetplayerlocation)
    (else
      (CallFunction|StartAtackCoolDown()))))

(event EventBeginPlay
  (|CallParentFunction)
  (bind _returnvalue (Utilities|Time|SetTimerbyEvent (delegate Custom|MoveRight) 0.01 true))
  (Variables|Movement|Timers|SetthMoveL/R _returnvalue))

(fn ConstructionScript
  (CallFunction|SetEnemyName() "NewEnumerator3")
  (switch Utilities|FlowControl|Switch|SwitchonEnemyNames (CallFunction|GetEnemyName())
    (:NewEnumerator2
      (Initilization|SetfMoveL/RDirection() true)
      (CallFunction|SetDetectionDirection() "NewEnumerator2"))
    (:NewEnumerator3
      (Initilization|SetfMoveL/RDirection() false)
      (CallFunction|SetDetectionDirection() "NewEnumerator3")))
  (|CallParentFunction))

(fn MoveLeft/Right()
  (params (fGetMoveDirection :type Float%20%28single-precision%29))
  (Pawn|Input|AddMovementInput "10000.000000, 0, 0" fGetMoveDirection true)
  (Movement|L/RMovementRange() fGetMoveDirection))

(fn L/RMovementRange()
  (params (fGetMoveDirection :type Float%20%28single-precision%29))
  (bind _fmovecounter (Variables|Movement|Floats|GetfMoveCounter))
  (if (> fGetMoveDirection 0.0)
    (bind _result (Math|Float|IncrementFloat _fmovecounter)
      (:%20%20
        (if (== _result (Variables|Movement|Floats|GetfMaxRightMove))
          (Utilities|Time|PauseTimerbyHandle (Variables|Movement|Timers|GetthMoveL/R) :!label _label)
          (Movement|ChangeMoveDirection() fGetMoveDirection))))
    (else
      (bind _result_2 (Math|Float|DecrementFloat _fmovecounter)
        (:%20%20
          (if (== _result_2 (Variables|Movement|Floats|GetfMaxLeftMove))
            (goto _label)))))))

(fn ChangeMoveDirection()
  (params (fGetMoveDirection :type Float%20%28single-precision%29))
  (if (< fGetMoveDirection 0.0)
    (Initilization|SetfMoveL/RDirection() false)
    (else
      (Initilization|SetfMoveL/RDirection() true)))
  (Utilities|Time|UnpauseTimerbyHandle (Variables|Movement|Timers|GetthMoveL/R)))

(fn SetfMoveL/RDirection()
  (params (bMoveLeft? :type Boolean))
  (if bMoveLeft?
    (Variables|Movement|Floats|SetfMoveL/RDirection -1.0)
    (else
      (Variables|Movement|Floats|SetfMoveL/RDirection 1.0))))

(fn SetChargetoLocation()
  (params (vGetPlayerLocation :type Vector))
  (Physics|AddImpulse (Variables|Character|GetCharacterMovement) (Math|Vector|MakeVector (- (.X (Math|Vector|BreakVector vGetPlayerLocation)) (.x (Transformation|GetWorldLocation (Variables|Default|GetCapsuleComponent)))) 0.0 5e+02) true)
  (Variables|Default|SetfAttackCoolDown 0.0)
  (Variables|Default|SetbCanAttack? false))