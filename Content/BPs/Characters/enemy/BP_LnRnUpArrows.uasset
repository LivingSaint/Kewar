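; Arrow enemy child Blueprint that jump-attacks when it detects the player above it.
; Construction sets the name to Left/Up Arrow, then derives move direction, detection direction and detection speed from it, with a Right/Up branch also present.
; A looping timer runs vertical detection, triggering the jump when attack is allowed and otherwise advancing the cooldown.
; BeginPlay also calls PauseMoveLR after starting the timer.
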(event Custom|DetectVerticalPlayer
  (if (CallFunction|GetbCanAttack())
    (bind (_bplayerdectected _vplayerlocation) (CallFunction|DetectionDirection() (CallFunction|GetvDetectionDirectionVertical())))
    (if _bplayerdectected
      (if (> (.Z (Math|Vector|BreakVector _vplayerlocation)) (.Z (Math|Vector|BreakVector (Transformation|GetWorldLocation (Variables|Default|GetCapsuleComponent)))))
        (CallFunction|JumpAttack())))
    (else
      (CallFunction|AttackCoolDown()))))

(event EventBeginPlay
  (|CallParentFunction)
  (bind _returnvalue (Utilities|Time|SetTimerbyEvent (delegate Custom|DetectVerticalPlayer) (CallFunction|GetDetectTime()) true))
  (Variables|Default|SetthDetectVertical _returnvalue)
  (CallFunction|PauseMoveL/R()))

(fn ConstructionScript
  (bind _eenemyname (CallFunction|GetEnemyName()))
  (|CallParentFunction)
  (CallFunction|SetEnemyName() "NewEnumerator5")
  (switch Utilities|FlowControl|Switch|SwitchonEnemyNames _eenemyname
    (:NewEnumerator5
      (CallFunction|SetMoveDirection() true))
    (:NewEnumerator6
      (CallFunction|SetMoveDirection() false)))
  (CallFunction|SetDetectionDirection() _eenemyname)
  (CallFunction|SetDetectionSpeed() 0.1))

(fn JumpAttack()
  (Character|Jump)
  (CallFunction|SetbCanAttack() false)
  (CallFunction|SetfAttackCoolDown() 0.0))