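; Toy car enemy that drives left or right along X toward the player, or away when inverse movement is set.
; While the tagged player is inside its sphere, a looping timer moves it and recalculates direction and walk speed from distance bands; leaving pauses the timer.
; It flags the player as above when nearly aligned in X.
; Helpers spawn a hazard attached to the sprite's socket and set a tiered boss speed increase.
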(event OnComponentEndOverlap(Sphere)
  (params (OverlappedComponent :type Primitive%20Component%20Object%20Reference) (OtherActor :type Actor%20Object%20Reference) (OtherComp :type Primitive%20Component%20Object%20Reference) (OtherBodyIndex :type Integer))
  (if (Actor|ActorHasTag OtherActor (CallFunction|GetnPlayerTag()))
    (CallFunction|SetMaxWalkSpeed() "NewEnumerator0" 0.0 0.0)
    (Utilities|Time|PauseTimerbyHandle (Variables|Default|Getth_moveto))))

(event OnComponentBeginOverlap(Sphere)
  (params (OverlappedComponent :type Primitive%20Component%20Object%20Reference) (OtherActor :type Actor%20Object%20Reference) (OtherComp :type Primitive%20Component%20Object%20Reference) (OtherBodyIndex :type Integer) (bFromSweep :type Boolean) (SweepResult :type Hit%20Result%20Structure%20%28by%20ref%29))
  (if (Actor|ActorHasTag OtherActor (CallFunction|GetnPlayerTag()))
    (bind _returnvalue (Utilities|Time|SetTimerbyEvent (delegate Custom|MoveMe) (CallFunction|GetfMoveSpeed()) true))
    (Variables|Default|Setth_moveto _returnvalue)))

(event Custom|MoveMe
  (CallFunction|MoveLeft/Right() (CallFunction|GetMoveDirection()))
  (CallFunction|CalculateMoveDirection())
  (CallFunction|CalculateMoveSpeed()))

(event EventBeginPlay
  (|CallParentFunction))

(event Collision|EventActorBeginOverlap
  (params (OtherActor :type Actor%20Object%20Reference)))

(fn ConstructionScript
  (|CallParentFunction))

(fn CalculateMoveDirection()
  (bind _returnvalue (Transformation|GetActorLocation))
  (bind _objplayercharacter (CallFunction|GetobjPlayerCharacter()))
  (bind _binversemovement_ (Variables|Default|GetbInverseMovement?))
  (bind _returnvalue_2 (Transformation|GetActorLocation _objplayercharacter))
  (if (Math|Float|InRange(Float) (- (.x _returnvalue_2) (.x _returnvalue)) -5.0 5.0)
    (ToyCar|Initiliaztion|Sets|SetbPlayerIsAbove() true)
    (else
      (ToyCar|Initiliaztion|Sets|SetbPlayerIsAbove() false)
      (if (> (.x _returnvalue_2) (.x _returnvalue))
        (if _binversemovement_
          (bind _output_get (Variables|Default|SetbMoveLeft? true :!label _label))
          (CallFunction|SetMoveDirection() _output_get)
          (else
            (bind _output_get_2 (Variables|Default|SetbMoveLeft? false :!label _label_2))
            (CallFunction|SetMoveDirection() _output_get_2)))
        (elif _binversemovement_
          (goto _label_2)
          (else
            (goto _label))))
      (Variables|Default|SetfDistanceToPlayer (- (.x _returnvalue_2) (.x _returnvalue)))
      (return))))

(fn CalculateMoveSpeed()
  (if (CallFunction|InRange() 2e+03)
    (if (Variables|Default|GetbInverseMovement?)
      (CallFunction|SetMaxWalkSpeed() "NewEnumerator2" 0.0 0.0)
      (else
        (CallFunction|SetMaxWalkSpeed() "NewEnumerator0" 0.0 0.0)))
    (elif (CallFunction|InRange() 1e+03)
      (if (Variables|Default|GetbInverseMovement?)
        (CallFunction|SetMaxWalkSpeed() "NewEnumerator1" 0.0 0.0)
        (else
          (CallFunction|SetMaxWalkSpeed() "NewEnumerator5" 0.0 0.0)))
      (elif (CallFunction|InRange() 5e+02)
        (if (Variables|Default|GetbInverseMovement?)
          (CallFunction|SetMaxWalkSpeed() "NewEnumerator1" 0.0 0.0)
          (else
            (CallFunction|SetMaxWalkSpeed() "NewEnumerator1" 0.0 0.0)))
        (elif (Variables|Default|GetbInverseMovement?)
          (CallFunction|SetMaxWalkSpeed() "NewEnumerator0" 0.0 0.0)
          (else
            (CallFunction|SetMaxWalkSpeed() "NewEnumerator2" 0.0 0.0)))))))

(fn GetbPlayerIsAbove()
  (return (Variables|Default|GetbPlayerIsAbove)))

(fn SetbPlayerIsAbove()
  (params (bPlayerIsAbove :type Boolean))
  (Variables|Default|SetbPlayerIsAbove bPlayerIsAbove))

(fn SpawnHazard()
  (params (SetHazzard :type Actor%20Class%20Reference))
  (bind _sprite (Variables|Default|GetSprite))
  (bind _returnvalue (Transformation|GetWorldTransform _sprite))
  (bind (_x _y _z) (Math|Vector|BreakVector (.location _returnvalue)))
  (bind _returnvalue_2 (Game|SpawnActorfromClass SetHazzard (Math|Transform|MakeTransform (Math|Vector|MakeVector _x _y (+ _z 2e+02)) (.rotation _returnvalue) "1.000000,1.000000,1.000000") "Undefined" 0 0))
  (bind _output_get (Variables|Default|SetobjHazardReference _returnvalue_2))
  (ToyCar|Initiliaztion|Sets|SetobjHazardReference() _output_get)
  (Transformation|AttachComponentToComponent _output_get _sprite (Utilities|Array|Get(acopy) (Transformation|GetAllSocketNames _sprite)) "SnapToTarget" "SnapToTarget" "SnapToTarget" false))

(fn SetobjHazardReference()
  (params (objHazardReference :type Actor%20Object%20Reference))
  (Variables|Default|SetobjHazardReference objHazardReference))

(fn GetobjHazardReference()
  (return (Variables|Default|GetobjHazardReference)))

(fn SetfBossSpeedIncrease()
  (params (NewParam :type Integer))
  (switch int NewParam
    (:0
      (Variables|Default|SetfBossSpeedIncrease 0.025))
    (:1
      (Variables|Default|SetfBossSpeedIncrease 0.05))
    (:2
      (Variables|Default|SetfBossSpeedIncrease 0.075))))

(fn GetfBossSpeedIncrease()
  (return (Variables|Default|GetfBossSpeedIncrease)))

(fn InRange()
  (params (SetfMaxDistance :type Float%20%28single-precision%29))
  (bind _fdistancetoplayer (Variables|Default|GetfDistanceToPlayer))
  (return (or (< _fdistancetoplayer (* SetfMaxDistance -1.0)) (> _fdistancetoplayer SetfMaxDistance))))

(fn SetbInverseMoveDirection()
  (params (bInverseMovement? :type Boolean))
  (Variables|Default|SetbInverseMovement? bInverseMovement?))