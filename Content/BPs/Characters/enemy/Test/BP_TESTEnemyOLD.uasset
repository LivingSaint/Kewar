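; An old test enemy Character for a side-view game, with prototype patrol, random jump and directional player detection.
; The construction script finds the Kerbo player, locks Y to zero and picks a trace direction from the enemy's arrow-named enum.
; Helpers handle timer-swapped left/right movement, line-trace detection and an attack cooldown counter.
; Most event logic, including timer setup and impulse lunges, is disconnected, leaving BeginPlay empty.
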(event Custom|MoveRight)

(event Custom|StartDetectingPlayer)

(event Custom|MoveLeft
  (CallFunction|MoveLeft/Right()TEST (Variables|Enemy|Movement|Left/Right|GetMoveDirectionTEST))
  (CallFunction|L/RMovementRange()TEST false))

(event EventBeginPlay)

(fn ConstructionScript
  (CallFunction|GetReferencetoPlayer())
  (Enemy|initilization|LockYAxis())
  (switch Utilities|FlowControl|Switch|SwitchonEnemyNames (Variables|Enemy|initilization|Enums|GeteEnemyName)
    (:NewEnumerator1
      (Variables|Enemy|initilization||Vector|SetvDetectionDirection "0, 0,1000.000000"))
    (:NewEnumerator4
      (Variables|Enemy|initilization||Vector|SetvDetectionDirection "0, 0,-1000.000000"))
    (:NewEnumerator2
      (Variables|Enemy|initilization||Vector|SetvDetectionDirection "-1000.000000, 0,0.000000"))
    (:NewEnumerator3
      (Variables|Enemy|initilization||Vector|SetvDetectionDirection "1000.000000, 0, 0"))))

(fn MoveLeft/Right()TEST
  (params (fLeft/RIght :type Float%20%28single-precision%29))
  (if (< fLeft/RIght 0.0)
    (Pawn|Input|AddMovementInput "10000.000000, 0, 0" fLeft/RIght true)
    (else
      (Pawn|Input|AddMovementInput "10000.000000, 0, 0" fLeft/RIght true)))
  (return))

(fn Jump()TEST
  (params (iSetMaxJumpChance :type Integer))
  (if (== (Math|Random|RandomIntegerinRange 0 iSetMaxJumpChance) 50)
    (Character|Jump)))

(fn L/RMovementRange()TEST
  (params (bMovingRight? :type Boolean))
  (bind _fmovecountertest (Variables|Enemy|Movement|Left/Right|GetfMoveCounterTEST))
  (if bMovingRight?
    (bind _result (Math|Float|IncrementFloat _fmovecountertest)
      (:%20%20
        (if (== _result (Variables|Enemy|Movement|Left/Right|GetfMaxMoveRangeTEST))
          (Utilities|Time|PauseTimerbyHandle (Variables|Enemy|Movement|Left/Right|GetthRightMoveTEST))
          (Variables|Enemy|Movement|Left/Right|SetMoveDirectionTEST -1.0)
          (Utilities|Time|UnpauseTimerbyHandle (Variables|Enemy|Movement|Left/Right|GetthLeftMoveTEST)))))
    (else
      (bind _result_2 (Math|Float|DecrementFloat _fmovecountertest)
        (:%20%20
          (if (== _result_2 (Variables|Enemy|Movement|Left/Right|GetfMinMoveRangeTEST))
            (Utilities|Time|PauseTimerbyHandle (Variables|Enemy|Movement|Left/Right|GetthLeftMoveTEST))
            (Variables|Enemy|Movement|Left/Right|SetMoveDirectionTEST 1.0)
            (Utilities|Time|UnpauseTimerbyHandle (Variables|Enemy|Movement|Left/Right|GetthRightMoveTEST))))))))

(fn LockYAxis()
  (bind _capsulecomponent (Variables|Collision|GetCapsuleComponent))
  (bind _returnvalue (Transformation|GetWorldLocation _capsulecomponent))
  (bind (_x _y _z) (Math|Vector|BreakVector _returnvalue))
  (Transformation|SetWorldLocation _capsulecomponent (Math|Vector|MakeVector _x 0.0 _z) false true))

(fn SetEnemyName()
  (params (eSetEnemyName1 :type EnemyNames%20Enum))
  (Variables|Enemy|initilization|Enums|SeteEnemyName eSetEnemyName1)
  (return))

(fn DetectionDirection()
  (params (vGetDetectionDirection :type Vector))
  (bind _capsulecomponent (Variables|Collision|GetCapsuleComponent))
  (bind _returnvalue (Transformation|GetWorldLocation _capsulecomponent))
  (bind (_outhit _returnvalue_2) (Collision|LineTraceByChannel _returnvalue (+ _returnvalue vGetDetectionDirection) "TraceTypeQuery1" false 0 "Persistent")) ; Up
  (if _returnvalue_2
    (Utilities|IsValid (.HitActor (Collision|BreakHitResult _outhit))
      (:Is%20Valid
        (if (Actor|ActorHasTag (.HitActor (Collision|BreakHitResult _outhit)) "Player")
          (return (Transformation|GetActorLocation (.HitActor (Collision|BreakHitResult _outhit))) _returnvalue_2))))
    (else
      (return "0, 0, 0" false))))

(fn GetEnemyName()
  (return (Variables|Enemy|initilization|Enums|GeteEnemyName)))

(fn SetDetectionDirection()
  (params (eGetEnemyName :type EnemyNames%20Enum))
  (switch Utilities|FlowControl|Switch|SwitchonEnemyNames eGetEnemyName
    (:NewEnumerator1
      (Variables|Enemy|initilization||Vector|SetvDetectionDirection "0.000000,0.000000,750.000000"))
    (:NewEnumerator4
      (Variables|Enemy|initilization||Vector|SetvDetectionDirection "0.000000, 0,-750.000000"))
    (:NewEnumerator2
      (Variables|Enemy|initilization||Vector|SetvDetectionDirection "-1000.000000, 0, 0"))
    (:NewEnumerator3
      (Variables|Enemy|initilization||Vector|SetvDetectionDirection "1000.000000, 0, 0"))))

(fn StartAtackCoolDown()
  (bind _fattackcooldown (Variables|Enemy|Floats|GetfAttackCoolDown))
  (if (== _fattackcooldown 1e+02)
    (Variables|Enemy|Bools|SetbCanAttack? true)
    (else
      (bind _result (Math|Float|IncrementFloat _fattackcooldown)
        (:%20%20
          (if (< _result 1e+02)
            (Variables|Enemy|Bools|SetbCanAttack? false)))))))

(fn GetReferencetoPlayer()
  (bind _outactors (Actor|GetAllActorsOfClass "/Game/BPs/Characters/Player/Kerbo.Kerbo_C"))
  (for _array_element _outactors
    (Utilities|IsValid _array_element
      (:Is%20Valid
        (bind _output_get (Variables|Default|SetobjPlayerRef _array_element))
        (Development|PrintString (Utilities|GetDisplayName _output_get))))))