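; BP_Enemy is a test enemy actor that slides to a target point when play begins.
; BeginPlay moves the root component over five seconds toward the world location of MovetoPoint, keeping its rotation.
; The construction script calls TESTLockYAxis, which teleports the root to zero world Y, pinning placement to the XZ plane.
; A Jump function is declared but empty.
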(event EventBeginPlay
  (Components|MoveComponentTo (Variables|Default|GetDefaultSceneRoot) (Transformation|GetWorldLocation (Variables|Default|GetMovetoPoint)) (Transformation|GetWorldRotation (Variables|Default|GetDefaultSceneRoot)) false false 5.0 false))

(fn ConstructionScript
  (CallFunction|TESTLockYAxis()))

(fn TESTLockYAxis()
  (bind _defaultsceneroot (Variables|Default|GetDefaultSceneRoot))
  (bind _returnvalue (Transformation|GetWorldLocation _defaultsceneroot))
  (bind (_x _y _z) (Math|Vector|BreakVector _returnvalue))
  (Transformation|SetWorldLocation _defaultsceneroot (Math|Vector|MakeVector _x 0.0 _z) false true))

(fn Jump())