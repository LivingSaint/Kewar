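; Test "Up Arrow" enemy, named as an old version, that leaps vertically to dodge a charging player.
; Player overlap with its box starts a looping timer that runs Dodge, line-tracing both ways along world X and adding an upward impulse if the traced player is charging.
; A player-tagged capsule hit unpauses that timer.
; The jump attack on players above, with its pause and cooldown, is disconnected and never runs.
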(event OnComponentBeginOverlap(Box)
  (params (OverlappedComponent :type Primitive%20Component%20Object%20Reference) (OtherActor :type Actor%20Object%20Reference) (OtherComp :type Primitive%20Component%20Object%20Reference) (OtherBodyIndex :type Integer) (bFromSweep :type Boolean) (SweepResult :type Hit%20Result%20Structure%20%28by%20ref%29))
  (if (Actor|ActorHasTag OtherActor "Player")
    (bind _returnvalue (Utilities|Time|SetTimerbyEvent (delegate Custom|JumpAttack) 0.1 true))
    (Variables|Default|SetthDetectUpwardPlayer _returnvalue)))

(event OnComponentHit(CapsuleComponent)
  (params (HitComponent :type Primitive%20Component%20Object%20Reference) (OtherActor :type Actor%20Object%20Reference) (OtherComp :type Primitive%20Component%20Object%20Reference) (NormalImpulse :type Vector :default "0, 0, 0") (Hit :type Hit%20Result%20Structure%20%28by%20ref%29))
  (if (Components|ComponentHasTag HitComponent "Player")
    (Utilities|Time|UnpauseTimerbyHandle (Variables|Default|GetthDetectUpwardPlayer))))

(event Custom|JumpAttack
  (CallFunction|Dodge() -1e+03 1e+03))

(event EventBeginPlay
  (|CallParentFunction))

(fn ConstructionScript
  (bind _eenemyname (CallFunction|GetEnemyName()))
  (switch Utilities|FlowControl|Switch|SwitchonEnemyNames _eenemyname
    (:NewEnumerator1
      (CallFunction|SetDetectionDirection() _eenemyname)
      (|CallParentFunction))))

(fn Jump()
  (Character|Jump)
  (Variables|Default|SetbCanAttack? false)
  (Variables|Default|SetfAttackCoolDown 0.0))

(fn Dodge()
  (params (fSetDodgeDetectionRangeL :type Float%20%28single-precision%29) (fSetDodgeDetectionRangeR :type Float%20%28single-precision%29))
  (bind _objplayerref (Variables|Default|GetobjPlayerRef))
  (bind _capsulecomponent (Variables|Default|GetCapsuleComponent))
  (bind _capsulecomponent_2 (Variables|Default|GetCapsuleComponent))
  (bind _returnvalue (Transformation|GetWorldLocation _capsulecomponent_2))
  (bind _returnvalue_2 (Transformation|GetWorldLocation _capsulecomponent))
  (Utilities|FlowControl|Sequence
    (:then_0
      (bind _outhit (Collision|LineTraceByChannel _returnvalue_2 (+ _returnvalue_2 (Math|Vector|MakeVector fSetDodgeDetectionRangeL 0.0 0.0)) "TraceTypeQuery1" false 0 "ForOneFrame"))
      (if (.bBlockingHit (Collision|BreakHitResult _outhit))
        (if (Actor|ActorHasTag (.HitActor (Collision|BreakHitResult _outhit)) "Player")
          (if (or (Variables|/Game/BPs/Characters/Player/Kerbo.Kerbo_C|GetbChargingLeft? _objplayerref) (Variables|/Game/BPs/Characters/Player/Kerbo.Kerbo_C|GetbChargingRight? _objplayerref)) :!label _label
            (Physics|AddImpulse (Variables|Character|GetCharacterMovement) "0, 0,1500.000000" true)))))
    (:then_1
      (bind _outhit_2 (Collision|LineTraceByChannel _returnvalue (+ _returnvalue (Math|Vector|MakeVector fSetDodgeDetectionRangeR 0.0 0.0)) "TraceTypeQuery1" false 0 "ForOneFrame"))
      (if (.bBlockingHit (Collision|BreakHitResult _outhit_2))
        (if (Actor|ActorHasTag (.HitActor (Collision|BreakHitResult _outhit_2)) "Player")
          (goto _label))))))