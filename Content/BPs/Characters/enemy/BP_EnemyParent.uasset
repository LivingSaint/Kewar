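; Base enemy for a side-scrolling game: locks to Y=0 on construction and fights the Kerbo player through directional hitbox contact.
; Arrow-type enemy names make every side vulnerable except the one pointed at, for the four single-arrow types.
; Player position and falling state determine hit side, either killing the enemy or damaging the player, with knockback either way.
; Also provides line-trace player detection, detection-direction setup and attack cooldown helpers, none called here.
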(event OnComponentBeginOverlap(HitBox)
  (params (OverlappedComponent :type Primitive%20Component%20Object%20Reference) (OtherActor :type Actor%20Object%20Reference) (OtherComp :type Primitive%20Component%20Object%20Reference) (OtherBodyIndex :type Integer) (bFromSweep :type Boolean) (SweepResult :type Hit%20Result%20Structure%20%28by%20ref%29))
  (bind _objplayercharacter (Variables|References|GetobjPlayerCharacter))
  (bind _objplayercharacter_2 (Variables|References|GetobjPlayerCharacter))
  (if (Actor|ActorHasTag OtherActor (Variables|References|GetnPlayerTag))
    (bind _ecanbedamagedlocations1 (CallFunction|HitLocation() (Transformation|GetActorLocation OtherActor)))
    (if (Parent|Gets|GetbCanbeDamagedDirection() _ecanbedamagedlocations1)
      (Development|PrintString "I died" true true "(R=1.000000,G=0.049562,B=0.000000,A=1.000000)")
      (Variables|Actions|SetbIsDead? true)
      (Default|CallIsDead true)
      (Components|Movement|StopMovementImmediately (Variables|/Script/Engine.Character|GetCharacterMovement _objplayercharacter))
      (Default|OnDamageKnockBack() _objplayercharacter (Transformation|GetWorldLocation (Variables|Collision|GetCapsuleComponent)))
      (Actor|DestroyActor)
      (else
        (Default|ReduceHealth() _objplayercharacter_2)
        (Default|OnDamageKnockBack() _objplayercharacter_2 (Transformation|GetWorldLocation (Variables|Collision|GetCapsuleComponent)))))))

(event EventBeginPlay
  (References|Set|OBJRefferences())
  (References|Set|SetnPlayerTag()))

(fn ConstructionScript
  (Parent|Initilization|LockYAxis())
  (Parent|Initilization|CanbeDamagedDirection()))

(fn AttackCoolDown()
  (bind _fattackcooldown (Variables|Actions|GetfAttackCoolDown))
  (bind _fmaxattackcooldown (LocalVariables|GetfMaxAttackCoolDown))
  (if (== _fattackcooldown _fmaxattackcooldown)
    (Parent|Sets|SetbCanAttack() true)
    (else
      (bind _result (Math|Float|IncrementFloat _fattackcooldown)
        (:%20%20
          (if (< _result _fmaxattackcooldown)
            (Parent|Sets|SetbCanAttack() false)))))))

(fn OBJRefferences()
  (Utilities|FlowControl|DoOnce false
    (:Completed
      (bind _outactors (Actor|GetAllActorsOfClass "/Game/BPs/Characters/Player/Kerbo.Kerbo_C"))
      (for _array_element _outactors
        (Variables|References|SetobjPlayerCharacter _array_element)))))

(fn LockYAxis()
  (bind _capsulecomponent (Variables|Collision|GetCapsuleComponent))
  (bind _returnvalue (Transformation|GetWorldLocation _capsulecomponent))
  (bind (_x _y _z) (Math|Vector|BreakVector _returnvalue))
  (Transformation|SetWorldLocation _capsulecomponent (Math|Vector|MakeVector _x 0.0 _z) false true))

(fn GetEnemyName()
  (return (Variables|Default|GeteEnemyName)))

(fn SetEnemyName()
  (params (eEnemyName :type EnemyNames%20Enum))
  (Variables|Default|SeteEnemyName eEnemyName))

(fn SetDetectionDirection()
  (params (eEnemyName :type EnemyNames%20Enum))
  (switch Utilities|FlowControl|Switch|SwitchonEnemyNames eEnemyName
    (:NewEnumerator1
      (Variables|Detection|SetvDetectionDirectionVertical "0, 0,1000.000000"))
    (:NewEnumerator4
      (Variables|Detection|SetvDetectionDirectionVertical "0, 0,-1000.000000"))
    (:NewEnumerator2
      (Variables|Detection|SetvDetectionDirectionHorizontal "-1000.000000, 0, 0"))
    (:NewEnumerator3
      (Variables|Detection|SetvDetectionDirectionHorizontal "1000.000000, 0, 0"))
    (:NewEnumerator5
      (Variables|Detection|SetvDetectionDirectionHorizontal "-1000.000000, 0,0.000000")
      (Variables|Detection|SetvDetectionDirectionVertical "0, 0,1000.000000" :!label _label))
    (:NewEnumerator6
      (Variables|Detection|SetvDetectionDirectionHorizontal "1000.000000, 0,0.000000")
      (goto _label))))

(fn GetbCanAttack()
  (return (Variables|Actions|GetbCanAttack)))

(fn GetvDetectionDirectionHorizontal()
  (return (Variables|Detection|GetvDetectionDirectionHorizontal)))

(fn DetectionDirection()
  (params (vDetectionDirection :type Vector))
  (bind _capsulecomponent (Variables|Collision|GetCapsuleComponent))
  (bind _returnvalue (Transformation|GetWorldLocation _capsulecomponent))
  (bind (_outhit _returnvalue_2) (Collision|LineTraceByChannel _returnvalue (+ _returnvalue vDetectionDirection) "TraceTypeQuery1" false 0 "ForOneFrame" true "(R=1.000000,G=0.000000,B=0.000000,A=1.000000)" "(R=0.000000,G=1.000000,B=0.000000,A=1.000000)" 5.0))
  (if _returnvalue_2
    (Utilities|IsValid (.HitActor (Collision|BreakHitResult _outhit))
      (:Is%20Valid
        (if (Actor|ActorHasTag (.HitActor (Collision|BreakHitResult _outhit)) "Player")
          (return true (Transformation|GetActorLocation (.HitActor (Collision|BreakHitResult _outhit))))
          (else
            _)))))
  (return false "-99999.000000,-99999.000000,-99999.000000"))

(fn SetfAttackCoolDown()
  (params (fAttackCoolDown :type Float%20%28single-precision%29))
  (Variables|Actions|SetfAttackCoolDown fAttackCoolDown))

(fn SetbCanAttack()
  (params (bCanAttack :type Boolean))
  (Variables|Actions|SetbCanAttack bCanAttack))

(fn GetobjPlayerCharacter
  (return (Variables|References|GetobjPlayerCharacter)))

(fn GetvDetectionDirectionVertical()
  (return (Variables|Detection|GetvDetectionDirectionVertical)))

(fn SetnPlayerTag()
  (Variables|References|SetnPlayerTag (Utilities|Array|Get(acopy) (Variables|/Script/Engine.Actor|GetTags (Variables|References|GetobjPlayerCharacter))))
  (return))

(fn GetnPlayerTag()
  (return (Variables|References|GetnPlayerTag)))

(fn HitLocation()
  (params (vPlayerLocation :type Vector))
  (bind (_x _y _z) (Math|Vector|BreakVector vPlayerLocation))
  (bind _capsulecomponent (Variables|Collision|GetCapsuleComponent))
  (bind _returnvalue (Transformation|GetWorldLocation _capsulecomponent))
  (bind (_x_2 _y_2 _z_2) (Math|Vector|BreakVector _returnvalue))
  (if (Math|Boolean|NotEqual(Boolean) (AI|Components|NavMovement|IsFalling (Variables|/Script/Engine.Character|GetCharacterMovement (References|Get|GetobjPlayerCharacter))) true)
    (if (> _x (+ _x_2 1e+01)) ; AttacledRight
      (Development|PrintString "Rdead")
      (LocalVariables|SeteCanBeDamagedLocations "NewEnumerator1")
      (return (LocalVariables|GeteCanBeDamagedLocations))
      (elif (< _x (- _x_2 1e+01)) ; AttackLeft
        (Development|PrintString "LDead")
        (LocalVariables|SeteCanBeDamagedLocations "NewEnumerator0")
        (return (LocalVariables|GeteCanBeDamagedLocations))))
    (elif (> _z (+ _z_2 1e+02)) ; AttackUp
      (Development|PrintString "UDead")
      (LocalVariables|SeteCanBeDamagedLocations "NewEnumerator2")
      (return (LocalVariables|GeteCanBeDamagedLocations))
      (elif (< _z (- _z_2 1e+02)) ; AttackUp
        (Development|PrintString "DDead")
        (LocalVariables|SeteCanBeDamagedLocations "NewEnumerator3")
        (return (LocalVariables|GeteCanBeDamagedLocations))))))

(fn CanbeDamagedDirection()
  (switch Utilities|FlowControl|Switch|SwitchonEnemyNames (Parent|Gets|GetEnemyName())
    (:NewEnumerator1
      (|UpArrowInitilization))
    (:NewEnumerator4
      (|DownArrowInitilization))
    (:NewEnumerator2
      (|LeftArrowInitilization))
    (:NewEnumerator3
      (|RightArrowInitilization))))

(fn GetbCanbeDamagedDirection()
  (params (ChooseDirection :type CanBeDamagedDirections%20Enum))
  (switch Utilities|FlowControl|Switch|SwitchonCanBeDamagedDirections ChooseDirection
    (:NewEnumerator0
      (LocalVariables|SetiArrayIndex 0))
    (:NewEnumerator1
      (LocalVariables|SetiArrayIndex 1))
    (:NewEnumerator2
      (LocalVariables|SetiArrayIndex 2))
    (:NewEnumerator3
      (LocalVariables|SetiArrayIndex 3)))
  (return (Utilities|Array|Get(acopy) (Variables|Actions|GetbCanBeDamagedDirection[]) (LocalVariables|GetiArrayIndex))))

(fn SetbCanbeDamagedDirection()
  (params (eDirection :type CanBeDamagedDirections%20Enum) (bSetCanBeDamaged :type Boolean))
  (switch Utilities|FlowControl|Switch|SwitchonCanBeDamagedDirections eDirection
    (:NewEnumerator0
      (LocalVariables|SetiChosenIndex 0))
    (:NewEnumerator1
      (LocalVariables|SetiChosenIndex 1))
    (:NewEnumerator2
      (LocalVariables|SetiChosenIndex 2))
    (:NewEnumerator3
      (LocalVariables|SetiChosenIndex 3)))
  (Utilities|Array|SetArrayElem (Variables|Actions|GetbCanBeDamagedDirection[]) (LocalVariables|GetiChosenIndex) bSetCanBeDamaged))

(fn GetbIsDead()
  (return (Variables|Actions|GetbIsDead?)))

(fn GetbIsEnvironment()
  (return (Variables|Default|GetbIsEnvironment)))

(fn SetbIsEnvironment()
  (params (bIsEnvironment :type Boolean))
  (Variables|Default|SetbIsEnvironment bIsEnvironment))