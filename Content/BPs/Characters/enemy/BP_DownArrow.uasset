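; BP_DownArrow is an enemy that lunges vertically down at a detected player, then returns to its original position.
; Unless flagged as environment, a looping timer started shortly after BeginPlay polls the inherited directional detection.
; A DoOnce gates MoveComponentTo down to the player's height and back, then attacking is disabled until cooldown logic runs.
; The construction script sets enemy type, detection direction and origin; floor detection is an unused stub.
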(event Custom|DetectFloor)

(event Custom|DetectPlayer
  (bind _capsulecomponent (Variables|Default|GetCapsuleComponent))
  (bind _capsulecomponent_2 (Variables|Default|GetCapsuleComponent))
  (bind _returnvalue (Transformation|GetWorldRotation _capsulecomponent_2))
  (bind _returnvalue_2 (Transformation|GetWorldLocation _capsulecomponent))
  (bind (_x _y) (Math|Vector|BreakVector _returnvalue_2))
  (if (CallFunction|GetbCanAttack())
    (bind (_bplayerdectected _vplayerlocation) (CallFunction|DetectionDirection() (CallFunction|GetvDetectionDirectionVertical())))
    (if _bplayerdectected
      (Utilities|FlowControl|DoOnce false :!label _label
        (:Completed
          (if (< (.Z (Math|Vector|BreakVector _vplayerlocation)) (.Z (Math|Vector|BreakVector _returnvalue_2)))
            (Components|MoveComponentTo _capsulecomponent_2 (Math|Vector|MakeVector _x _y (.Z (Math|Vector|BreakVector _vplayerlocation))) _returnvalue false false 0.2 false)
            (Utilities|FlowControl|Delay 0.2)
            (Components|MoveComponentTo (Variables|Default|GetCapsuleComponent) (Variables|Default|GetvOriginalLocation) _returnvalue false false 0.2 false)
            (CallFunction|SetfAttackCoolDown() 0.0)
            (CallFunction|SetbCanAttack() false)))))
    (else
      (CallFunction|AttackCoolDown())
      (goto _label Reset))))

(event EventBeginPlay
  (|CallParentFunction)
  (Utilities|FlowControl|Delay 0.2)
  (if (not (CallFunction|GetbIsEnvironment()))
    (bind _returnvalue (Utilities|Time|SetTimerbyEvent (delegate Custom|DetectPlayer) 0.1 true))
    (Variables|Default|SetthDetectPlayer _returnvalue)))

(fn ConstructionScript
  (CallFunction|SetEnemyName() "NewEnumerator4")
  (|CallParentFunction)
  (CallFunction|SetDetectionDirection() (CallFunction|GetEnemyName()))
  (CallFunction|SetOriginalLocation))

(fn SetOriginalLocation
  (Variables|Default|SetvOriginalLocation (Transformation|GetWorldLocation (Variables|Default|GetCapsuleComponent))))