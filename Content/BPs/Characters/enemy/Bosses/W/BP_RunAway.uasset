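; Boss-folder enemy child that moves in inverted direction, as a runaway, and jumps at floor gaps until it dies.
; A looping timer traces for floor ahead; on a gap it pauses and calls AttackPlayer toward a landing point found by traces at stepped ranges.
; On death it gets launched, switches LockYAxis environment, then polls traces for a "BossFloors" actor, matched by display name, to switch again and stop.
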(event OnComponentHit(CapsuleComponent)
  (params (HitComponent :type Primitive%20Component%20Object%20Reference) (OtherActor :type Actor%20Object%20Reference) (OtherComp :type Primitive%20Component%20Object%20Reference) (NormalImpulse :type Vector :default "0, 0, 0") (Hit :type Hit%20Result%20Structure%20%28by%20ref%29))
  (if (Math|Boolean|NotEqual(Boolean) (Variables|Default|GetbCanJump?) false)
    (Utilities|Time|UnpauseTimerbyHandle (Variables|Default|GetthTest))
    (Variables|Default|SetbCanJump? true)))

(event Custom|Test
  (bind (_detectfloorbelow _detectfloorinfront) (Utilities|CheckFloorRange))
  (if (CallFunction|GetbIsDead())
    (Utilities|Time|PauseTimerbyHandle (Variables|Default|GetthTest))
    (else
      (bind _outhit (Collision|LineTraceByChannel _detectfloorbelow _detectfloorinfront "TraceTypeQuery1" false 0 "None"))
      (if (and (Math|Boolean|Equal(Boolean) (.bBlockingHit (Collision|BreakHitResult _outhit)) false) (Variables|Default|GetbCanJump?))
        (Utilities|Time|PauseTimerbyHandle (Variables|Default|GetthTest))
        (bind _vjumptolocation (CallFunction|FindJumptoLocation()))
        (CallFunction|AttackPlayer() 3e+02 _vjumptolocation)
        (Variables|Default|SetbCanJump? false)))))

(event Custom|OnDeath
  (params (NewParam :type Boolean))
  (Development|PrintString "Dead")
  (Physics|AddImpulse (Variables|Character|GetCharacterMovement) "750.000000,0.000000,500.000000" true)
  (bind _returnvalue (Utilities|Time|SetTimerbyEvent (delegate Custom|CustomEvent_0) 0.25 true))
  (Variables|Default|SetNewVar_0 _returnvalue)
  (Utilities|FlowControl|Delay 0.5)
  (CallFunction|LockYAxis "NewEnumerator5" (Variables|Default|GetCapsuleComponent) (Variables|Default|GetiLayerLevel)))

(event Custom|CustomEvent_0
  (bind (_detectfloorbelow _detectfloorinfront) (Utilities|CheckFloorRange))
  (bind _outhit (Collision|LineTraceByChannel (- _detectfloorbelow "0,300.000000,0.000000") (- _detectfloorinfront "0,300.000000,250.000000") "TraceTypeQuery1" false 0 "Persistent"))
  (if (Utilities|Enum|Equal(Enum) (Utilities|GetDisplayName (.HitActor (Collision|BreakHitResult _outhit))) "BossFloors")
    (CallFunction|LockYAxis "NewEnumerator4" (Variables|Default|GetCapsuleComponent) (Variables|Default|GetiLayerLevel))
    (Utilities|Time|ClearandInvalidateTimerbyHandle (Variables|Default|GetNewVar_0))
    (Components|Movement|StopMovementImmediately (Variables|Character|GetCharacterMovement))))

(event EventBeginPlay
  (|CallParentFunction)
  (EventDispatchers|BindEventtoIsDead (delegate Custom|OnDeath))
  (bind _returnvalue (Utilities|Time|SetTimerbyEvent (delegate Custom|Test) 0.25 true))
  (Variables|Default|SetthTest _returnvalue))

(event Collision|EventActorBeginOverlap
  (params (OtherActor :type Actor%20Object%20Reference)))

(fn ConstructionScript
  (|CallParentFunction)
  (CallFunction|SetbInverseMoveDirection() true)
  (CallFunction|SetbUseParentDestory() false))

(fn FindJumptoLocation()
  (bind _bxrange (LocalVariables|GetbXRange))
  (bind _fjumprangereduction (Variables|Default|GetfJumpRangeReduction))
  (bind _returnvalue (/ _bxrange _fjumprangereduction))
  (bind (_detectfloorbelow _detectfloorinfront) (Utilities|CheckJumpRange _returnvalue))
  (bind _index (Utilities|FlowControl|ForLoopwithBreak 0 5 :!label _label)
    (:LoopBody
      (LocalVariables|SetiLocalIndex _index)
      (bind _outhit (Collision|LineTraceByChannel _detectfloorbelow _detectfloorinfront "TraceTypeQuery1" false 0 "Persistent"))
      (if (.bBlockingHit (Collision|BreakHitResult _outhit))
        (goto _label Break)
        (else
          (Math|Float|DecrementFloat (Variables|Default|GetfJumpRangeReduction)))))
    (:Completed
      (return (.Location (Collision|BreakHitResult _outhit))))))