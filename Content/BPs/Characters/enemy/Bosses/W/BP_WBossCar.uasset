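; BP_WBossCar is a W boss car whose WBoss component bounces up against overhead surfaces and smashes breakables.
; A looping one-second timer traces upward from the capsule, sweeps WBoss to any blocking hit, then sweeps it back to the Billboard's position after a brief delay.
; WBoss hits destroy actors tagged Breakable, while the Sprite hit event is empty.
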(event OnComponentHit(WBoss)
  (params (HitComponent :type Primitive%20Component%20Object%20Reference) (OtherActor :type Actor%20Object%20Reference) (OtherComp :type Primitive%20Component%20Object%20Reference) (NormalImpulse :type Vector :default "0, 0, 0") (Hit :type Hit%20Result%20Structure%20%28by%20ref%29))
  (if (Actor|ActorHasTag OtherActor "Breakable")
    (Actor|DestroyActor OtherActor)))

(event OnComponentHit(Sprite)
  (params (HitComponent :type Primitive%20Component%20Object%20Reference) (OtherActor :type Actor%20Object%20Reference) (OtherComp :type Primitive%20Component%20Object%20Reference) (NormalImpulse :type Vector :default "0, 0, 0") (Hit :type Hit%20Result%20Structure%20%28by%20ref%29)))

(event Custom|Bounce
  (bind _wboss (Variables|Default|GetWBoss))
  (bind _capsulecomponent (Variables|Default|GetCapsuleComponent))
  (bind _returnvalue (Transformation|GetWorldLocation _capsulecomponent))
  (bind _outhit (Collision|LineTraceByChannel _returnvalue (+ _returnvalue "0, 0,1250.000000") "TraceTypeQuery1" false 0 "ForOneFrame"))
  (if (.bBlockingHit (Collision|BreakHitResult _outhit))
    (Transformation|SetWorldLocation _wboss (.Location (Collision|BreakHitResult _outhit)) true false)
    (Utilities|FlowControl|Delay 0.25)
    (Transformation|SetWorldLocation _wboss (Transformation|GetWorldLocation (Variables|Default|GetBillboard)) true false)))

(event EventBeginPlay
  (|CallParentFunction)
  (bind _returnvalue (Utilities|Time|SetTimerbyEvent (delegate Custom|Bounce) 1.0 true))
  (Variables|Default|SetthBounceTime _returnvalue))

(fn ConstructionScript
  (|CallParentFunction))