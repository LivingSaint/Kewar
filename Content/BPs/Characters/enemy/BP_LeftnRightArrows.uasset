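; Arrow enemy character that patrols horizontally and leaps at the player when detected.
; Construction sets initial direction and detection from the enemy name; looping timers then drive movement and detection if detection is enabled.
; An optional step-counter range reverses the patrol at its limits.
; Detection triggers a delayed impulse toward the player's X position, followed by cooldown, and capsule overlap with the player reports a hit.
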(event OnComponentBeginOverlap(CapsuleComponent)
  (params (OverlappedComponent :type Primitive%20Component%20Object%20Reference) (OtherActor :type Actor%20Object%20Reference) (OtherComp :type Primitive%20Component%20Object%20Reference) (OtherBodyIndex :type Integer) (bFromSweep :type Boolean) (SweepResult :type Hit%20Result%20Structure%20%28by%20ref%29))
  (if (Actor|ActorHasTag OtherActor (CallFunction|GetnPlayerTag()))
    (CallFunction|HitLocation() (Transformation|GetActorLocation OtherActor))))

(event Custom|StartMoving
  (Movement|MoveLeft/Right() (Initilization|Gets|GetMoveDirection())))

(event Custom|DetectPlayerHorizontal
  (if (CallFunction|GetbCanAttack())
    (bind (_bplayerdectected _vplayerlocation) (CallFunction|DetectionDirection() (CallFunction|GetvDetectionDirectionHorizontal())))
    (if _bplayerdectected
      (Utilities|FlowControl|Delay 1.0)
      (Actions|AttackPlayer() _vplayerlocation))
    (else
      (CallFunction|AttackCoolDown()))))

(event EventBeginPlay
  (|CallParentFunction)
  (if (CallFunction|GetbUseDetection())
    (bind _returnvalue (Utilities|Time|SetTimerbyEvent (delegate Custom|DetectPlayerHorizontal) (Variables|Detection|GetfDetectTime) true))
    (Variables|Detection|SetthDectectPlayer _returnvalue)
    (bind _returnvalue_2 (Utilities|Time|SetTimerbyEvent (delegate Custom|StartMoving) (CallFunction|GetfMoveSpeed()) true))
    (Variables|Movement|SetthMoveL/R _returnvalue_2)))

(fn ConstructionScript
  (bind _eenemyname (CallFunction|GetEnemyName()))
  (CallFunction|SetEnemyName() "NewEnumerator2")
  (|CallParentFunction)
  (switch Utilities|FlowControl|Switch|SwitchonEnemyNames _eenemyname
    (:NewEnumerator2
      (Initilization|Sets|SetMoveDirection() true))
    (:NewEnumerator3
      (Initilization|Sets|SetMoveDirection() false)))
  (CallFunction|SetDetectionDirection() _eenemyname)
  (Initilization|Sets|SetDetectionSpeed() 0.1))

(fn MoveLeft/Right()
  (params (fMoveDirection :type Float%20%28single-precision%29))
  (Pawn|Input|AddMovementInput (Variables|LeftnRight|Vectors|GetvMovementSpeed) fMoveDirection true)
  (if (Variables|LeftnRight|Bools|GetbHsaRange)
    (Movement|MovementRange() fMoveDirection)))

(fn MovementRange()
  (params (fMoveDirection :type Float%20%28single-precision%29))
  (bind _fmovecounter (Variables|Movement|GetfMoveCounter))
  (if (> fMoveDirection 0.0)
    (bind _result (Math|Float|IncrementFloat _fmovecounter)
      (:%20%20
        (if (== _result (LocalVariables|GetfMaxRightMove))
          (Utilities|Time|PauseTimerbyHandle (Variables|Movement|GetthMoveL/R) :!label _label)
          (Movement|ChangeMoveDirection() fMoveDirection)
          (return))))
    (else
      (bind _result_2 (Math|Float|DecrementFloat _fmovecounter)
        (:%20%20
          (if (== _result_2 (LocalVariables|GetfMaxMoveLeft))
            (goto _label)))))))

(fn ChangeMoveDirection()
  (params (fMoveDirection :type Float%20%28single-precision%29))
  (if (< fMoveDirection 0.0)
    (Initilization|Sets|SetMoveDirection() false)
    (else
      (Initilization|Sets|SetMoveDirection() true)))
  (Utilities|Time|UnpauseTimerbyHandle (Variables|Movement|GetthMoveL/R)))

(fn SetMoveDirection()
  (params (bMoveLeft? :type Boolean))
  (if bMoveLeft?
    (Variables|Movement|SetfMoveDirection -1.0)
    (else
      (Variables|Movement|SetfMoveDirection 1.0))))

(fn AttackPlayer()
  (params (vPlayerLocation :type Vector))
  (Physics|AddImpulse (Variables|Character|GetCharacterMovement) (Math|Vector|MakeVector (- (.X (Math|Vector|BreakVector vPlayerLocation)) (.x (Transformation|GetWorldLocation (Variables|Default|GetCapsuleComponent)))) 0.0 5e+02) true)
  (CallFunction|SetfAttackCoolDown() 0.0)
  (CallFunction|SetbCanAttack() false))

(fn GetMoveDirection()
  (return (Variables|Movement|GetfMoveDirection)))

(fn PauseMoveL/R()
  (Utilities|Time|PauseTimerbyHandle (Variables|Movement|GetthMoveL/R)))

(fn SetDetectionSpeed()
  (params (fDetectTime :type Float%20%28single-precision%29))
  (Variables|Detection|SetfDetectTime fDetectTime))

(fn GetDetectTime()
  (return (Variables|Detection|GetfDetectTime)))

(fn SetvMovementSpeed()
  (params (vMovementSpeed :type Vector))
  (Variables|LeftnRight|Vectors|SetvMovementSpeed vMovementSpeed))

(fn GetfMoveSpeed()
  (return (Variables|Movement|GetfMovementSpeed)))

(fn SetfMoveSpeed()
  (params (fMovementSpeed :type Float%20%28single-precision%29))
  (Variables|Movement|SetfMovementSpeed fMovementSpeed))

(fn GetvMoveSpeed()
  (return (Variables|LeftnRight|Vectors|GetvMovementSpeed)))

(fn SetVMoveSpeed()
  (params (vMovementSpeed :type Vector))
  (Variables|LeftnRight|Vectors|SetvMovementSpeed vMovementSpeed))