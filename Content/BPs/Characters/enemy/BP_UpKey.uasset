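; Up-arrow key enemy, built on a parent enemy class, that jump-attacks players above it and dodges their sideways charges.
; Looping timers poll both behaviours, with detection direction set from the enemy name at construction.
; Detecting a higher player pauses that timer, jumps and resets the attack cooldown.
; Line traces along world X find the player, and an upward velocity impulse dodges left or right charges.
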(event Custom|DetectDodge
  (CallFunction|Dodge() -1e+03 1e+03))

(event Custom|DetectAbovePlayer
  (if (CallFunction|GetbCanAttack())
    (bind (_bplayerdectected _vplayerlocation) (CallFunction|DetectionDirection() (CallFunction|GetvDetectionDirection())))
    (if _bplayerdectected
      (if (> (.Z (Math|Vector|BreakVector _vplayerlocation)) (.Z (Math|Vector|BreakVector (Transformation|GetWorldLocation (Variables|Default|GetCapsuleComponent)))))
        (Utilities|Time|PauseTimerbyHandle (Variables|Attack|GetthJumpAttack))
        (CallFunction|JumpAttack())))
    (else
      (CallFunction|AttackCoolDown()))))

(event EventBeginPlay
  (|CallParentFunction)
  (bind _returnvalue (Utilities|Time|SetTimerbyEvent (delegate Custom|DetectDodge) 0.1 true))
  (Variables|Dodge|SetthDodge _returnvalue)
  (bind _returnvalue_2 (Utilities|Time|SetTimerbyEvent (delegate Custom|DetectAbovePlayer) 0.1 true))
  (Variables|Attack|SetthJumpAttack _returnvalue_2))

(fn ConstructionScript
  (bind _eenemyname (CallFunction|GetEnemyName()))
  (|CallParentFunction)
  (CallFunction|SetEnemyName() "NewEnumerator1")
  (switch Utilities|FlowControl|Switch|SwitchonEnemyNames _eenemyname
    (:NewEnumerator1
      (CallFunction|SetDetectionDirection() _eenemyname))))

(fn Dodge()
  (params (fDodgeDirectionL :type Float%20%28single-precision%29) (fDodgeDirectionR :type Float%20%28single-precision%29))
  (bind _objplayercharacter (CallFunction|GetobjPlayerCharacter))
  (bind _capsulecomponent (Variables|Default|GetCapsuleComponent))
  (bind _capsulecomponent_2 (Variables|Default|GetCapsuleComponent))
  (bind _returnvalue (Transformation|GetWorldLocation _capsulecomponent_2))
  (bind _returnvalue_2 (Transformation|GetWorldLocation _capsulecomponent))
  (Utilities|FlowControl|Sequence
    (:then_0
      (bind (_outhit _returnvalue_3) (Collision|LineTraceByChannel _returnvalue_2 (+ _returnvalue_2 (Math|Vector|MakeVector fDodgeDirectionL 0.0 0.0)) "TraceTypeQuery1" false 0 "ForOneFrame"))
      (if _returnvalue_3
        (if (Actor|ActorHasTag (.HitActor (Collision|BreakHitResult _outhit)) "Player")
          (if (or (Variables|/Game/BPs/Characters/Player/Kerbo.Kerbo_C|GetbChargingLeft? _objplayercharacter) (Variables|/Game/BPs/Characters/Player/Kerbo.Kerbo_C|GetbChargingRight? _objplayercharacter)) :!label _label
            (Physics|AddImpulse (Variables|Character|GetCharacterMovement) "0, 0,1500.000000" true)))))
    (:then_1
      (bind (_outhit_2 _returnvalue_4) (Collision|LineTraceByChannel _returnvalue (+ _returnvalue (Math|Vector|MakeVector fDodgeDirectionR 0.0 0.0)) "TraceTypeQuery1" false 0 "ForOneFrame"))
      (if _returnvalue_4
        (if (Actor|ActorHasTag (.HitActor (Collision|BreakHitResult _outhit_2)) "Player")
          (goto _label))))))

(fn JumpAttack()
  (Character|Jump)
  (CallFunction|SetbCanAttack() false)
  (CallFunction|SetfAttackCoolDown() 0.0))