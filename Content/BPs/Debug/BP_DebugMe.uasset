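; Debug helper that reports a bug at a chosen severity by printing the affected object's display name and function name.
; DebugMe switches on the severity level to build the message, prefixing High with "error:" and Medium with "warning:", while Low has no prefix.
; The Medium message is worded as a "low level" bug, matching Low.
; All three levels share one optional print for additional notes.
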(fn DebugMe()
  (params (eSetBugLevel :type BugLevel%20Enum) (sGetDisplayName :type String) (sFunctionName :type String) (bAddAdditionalNotes :type Boolean) (sAdditionalNotes :type String))
  (switch Utilities|FlowControl|Switch|SwitchonBugLevel eSetBugLevel
    (:NewEnumerator0
      (Development|PrintString 0 (Utilities|String|Append "error: A high level Bug has occoured in:" "[" (Utilities|String|Append "   " sGetDisplayName "   ") "]" " 
The following function has been affected:" "[" (Utilities|String|Append "   " sFunctionName "   ") "]") false true "(R=1.000000,G=0.015401,B=0.000000,A=1.000000)")
      (if bAddAdditionalNotes
        (Development|PrintString 0 (Utilities|String|Append "Additional Notes:" sAdditionalNotes) :!label _label)))
    (:NewEnumerator1
      (Development|PrintString 0 (Utilities|String|Append "warning: A low level Bug has occoured in:" "[" (Utilities|String|Append "   " sGetDisplayName "   ") "]" " 
The following function has been affected:" "[" (Utilities|String|Append "   " sFunctionName "   ") "]") true true "(R=1.000000,G=0.619745,B=0.000000,A=1.000000)")
      (if bAddAdditionalNotes
        (goto _label)))
    (:NewEnumerator2
      (Development|PrintString 0 (Utilities|String|Append "A low level Bug has occoured in:" "[" (Utilities|String|Append "   " sGetDisplayName "   ") "]" " 
The following function has been affected:" "[" (Utilities|String|Append "   " sFunctionName "   ") "]") true false "(R=0.000000,G=0.660000,B=1.000000,A=1.000000)" 1e+01)
      (if bAddAdditionalNotes
        (goto _label)))))